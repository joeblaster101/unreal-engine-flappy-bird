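; Game-logic Blueprint for a bird game that runs the round and keeps score.
; On BeginPlay it shows the main menu, starts a looping timer that accumulates time alive, and immediately calls StartRound.
; StartRound possesses the first BP_bird, restores normal time dilation and resets time alive.
; CoinDelta increments coins, and tally multiplies them by time alive for the score, updating the high score.
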(event `StartRound`
  ;[0 0.625 1] round start
  (bind _outactors (`GameplayStatics.GetAllActorsOfClass` "/Game/blueprints/BP_bird.BP_bird_C"))
  (`Controller.Possess` (`GameplayStatics.GetPlayerController` 0) (`|GetArrayItem` _outactors))
  (`GameplayStatics.SetGlobalTimeDilation` 1.0)
  (set `self.TimeAlive` 0.0))

(event `self.ReceiveBeginPlay`
  ;[0 0.6016 1] begin game logic
  (`KismetSystemLibrary.K2_SetTimer` null "time alive" 0.1 true)
  (bind _returnvalue (`|CreateWidget` "/Game/blueprints/WB_mainMenu.WB_mainMenu_C"))
  (bind _returnvalue_2 (`UserWidget.AddToPlayerScreen` _returnvalue 0))
  ;[1 0 0.5625] Debug
  (`self.StartRound`)
  (if _returnvalue_2
    (`KismetSystemLibrary.PrintString` (`self.it works`))))

(event `tally`
  ;[0 1 0.3438] round end
  ;;[1 0.07031 0] score
  (bind _output_get (set `self.score` (`KismetMathLibrary.FTrunc` (* (`self.coin`) (`self.TimeAlive`)))))
  (if (>= _output_get (`self.HightScore`))
    (set `self.HightScore` _output_get)))

(fn `CoinDelta`
  ;[1 0 0.9844] Comment
  (bind _result (`/Engine/EditorBlueprintResources/StandardMacros.IncrementInt` (`self.coin`))
    (:`  `
      ;;[0 0.03906 1] debug
      (`KismetSystemLibrary.PrintString` (`KismetStringLibrary.Concat_StrStr` "coins" (`KismetStringLibrary.Conv_IntToString` _result))))))

(fn `time alive`
  ;[0.9219 1 0] TimealiveScore
  (bind _output_get (set `self.TimeAlive` (+ (`self.TimeAlive`) 0.1)))
  ;;[0.7109 1 0] debug
  (`KismetSystemLibrary.PrintString` (`KismetStringLibrary.Concat_StrStr` "time" (`KismetStringLibrary.Conv_DoubleToString` _output_get)) true true (struct :`R` 0.146897 :`G` 1.0 :`A` 1.0) 0.1))

(fn `UserConstructionScript`)