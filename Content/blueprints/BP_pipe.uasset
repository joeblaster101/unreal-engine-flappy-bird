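; BP_pipe is a Flappy Bird-style pipe obstacle that kills BP_bird when it hits the Top or Bottom component.
; On BeginPlay it sets a limited lifespan and spawns a BP_coin at CoinSpawn with a random height offset.
; When the bird first overlaps Box, a DoOnce-gated spawn places the next BP_pipe at ObsticalLocation with random vertical variation, so the obstacles chain endlessly.
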(event `self.ReceiveBeginPlay`
  (bind (_returnvalue_location _returnvalue_rotation _returnvalue_scale) (`KismetMathLibrary.BreakTransform` (`SceneComponent.K2_GetComponentToWorld` (`self.coin spawn`))))
  (bind (_x _y _z) (`KismetMathLibrary.BreakVector3f` _returnvalue_location))
  ;[0.7812 1 0] kill pipe
  (`self.SetLifeSpan` 30.0)
  (`|SpawnActorFromClass` "/Game/blueprints/BP_coin.BP_coin_C" (`KismetMathLibrary.MakeTransform` (`KismetMathLibrary.MakeVector` _x _y (+ (`KismetMathLibrary.RandomFloatInRange` -120.0 120.0) _z)) _returnvalue_rotation _returnvalue_scale) "Undefined" "MultiplyWithRoot" null null))

(event `self.top.OnComponentHit`
  (params (HitComponent :type "PrimitiveComponent Object Reference") (OtherActor :type "Actor Object Reference") (OtherComp :type "PrimitiveComponent Object Reference") (NormalImpulse :type "Vector Structure") (Hit :type "HitResult Structure (by ref)"))
  ;[1 0 0.1641] it kill
  (bind _asbp_bird (cast `/Game/blueprints/BP_bird` OtherActor))
  (`/Game/blueprints/BP_bird.die` _asbp_bird))

(event `self.bottom.OnComponentHit`
  (params (HitComponent :type "PrimitiveComponent Object Reference") (OtherActor :type "Actor Object Reference") (OtherComp :type "PrimitiveComponent Object Reference") (NormalImpulse :type "Vector Structure") (Hit :type "HitResult Structure (by ref)"))
  ;[1 0 0.1641] it kill
  (bind _asbp_bird (cast `/Game/blueprints/BP_bird` OtherActor))
  (`/Game/blueprints/BP_bird.die` _asbp_bird))

(event `self.Box.OnComponentBeginOverlap`
  (params (OverlappedComponent :type "PrimitiveComponent Object Reference") (OtherActor :type "Actor Object Reference") (OtherComp :type "PrimitiveComponent Object Reference") (OtherBodyIndex :type Integer) (bFromSweep :type Boolean) (SweepResult :type "HitResult Structure (by ref)"))
  (bind (_returnvalue_location _returnvalue_rotation _returnvalue_scale) (`KismetMathLibrary.BreakTransform` (`SceneComponent.K2_GetComponentToWorld` (`self.obstical location`))))
  (bind (_x _y _z) (`KismetMathLibrary.BreakVector3f` _returnvalue_location))
  ;[1 0 0.4687] spawn pip
  (cast `/Game/blueprints/BP_bird` OtherActor)
  (`/Engine/EditorBlueprintResources/StandardMacros.DoOnce` false
    (:`Completed`
      (`|SpawnActorFromClass` "BP_pipe_C" (`KismetMathLibrary.MakeTransform` (`KismetMathLibrary.MakeVector` _x _y (+ (`KismetMathLibrary.RandomFloatInRange` -100.0 100.0) _z)) _returnvalue_rotation _returnvalue_scale) "Undefined" "MultiplyWithRoot" null null))))

(fn `UserConstructionScript`)